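; Enemy AI controller that patrols BP_Waypoint actors until its perception detects something, then switches to pursuit.
; Successful move completions advance a looping index through the waypoints, in GetAllActorsOfClass order, after a short delay.
; The first perception update with actors stops movement and sets a chase state, which never resets.
; Chasing issues moves toward the updated perceived actors, stopping at any within close range.
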(event OnPerceptionUpdated(AIPerception)
  (params (UpdatedActors :type Array%20of%20Actor%20Object%20References))
  ;[1 0.8127 0.7524] Verificar estado ruta
  (if (== (Variables|Default|GetState) 0)
    (if (>= (Utilities|Array|Length UpdatedActors) 1)
      (Variables|Default|SetState 1)
      (AI|Navigation|StopMovement)
      ;[0.9949 0.6783 1] Hacer rutas
      (if (== (Variables|Default|GetState) 0)
        (Utilities|FlowControl|RetriggerableDelay 0.2)
        (bind _outactors (Actor|GetAllActorsOfClass "/Game/Blueprints/BP_Waypoint.BP_Waypoint_C"))
        (Variables|Default|SetCurrentWaypoint (Utilities|Array|Get(acopy) _outactors (Math|Integer|%(Integer) (+ (Variables|Default|GetCurrentPointID) 1) (Utilities|Array|Length _outactors))))
        (Variables|Default|SetCurrentPointID (Math|Integer|%(Integer) (+ (Variables|Default|GetCurrentPointID) 1) (Utilities|Array|Length _outactors)))
        (AI|Navigation|MovetoActor (Variables|Default|GetCurrentWaypoint) -1.0 true true true 0)
        (elif (== (Variables|Default|GetState) 1)
          (bind _returnvalue (Utilities|GetAIController)
            (:Is%20Valid
              (bind _array_element (Utilities|Array|ForEachLoopwithBreak UpdatedActors :!label _label)
                (:LoopBody
                  (if (<= (Math|Vector|VectorLength (- (Transformation|GetActorLocation (Pawn|GetControlledPawn _returnvalue)) (Transformation|GetActorLocation _array_element))) 1e+02)
                    (goto _label Break)
                    (else
                      (AI|Navigation|MovetoActor _array_element -1.0 true true true 0))))))))))))

(event Custom|NextRoute
  (params (RequestID :type AI%20Request%20ID%20Structure) (Result :type EPathFollowingResult%20Enum :default "Success"))
  ;[0.9949 0.6783 1] Hacer rutas
  (switch Utilities|FlowControl|Switch|SwitchonEPathFollowingResult Result
    (:Success
      (if (== (Variables|Default|GetState) 0)
        (Utilities|FlowControl|RetriggerableDelay 0.2)
        (bind _outactors (Actor|GetAllActorsOfClass "/Game/Blueprints/BP_Waypoint.BP_Waypoint_C"))
        (Variables|Default|SetCurrentWaypoint (Utilities|Array|Get(acopy) _outactors (Math|Integer|%(Integer) (+ (Variables|Default|GetCurrentPointID) 1) (Utilities|Array|Length _outactors))))
        (Variables|Default|SetCurrentPointID (Math|Integer|%(Integer) (+ (Variables|Default|GetCurrentPointID) 1) (Utilities|Array|Length _outactors)))
        (AI|Navigation|MovetoActor (Variables|Default|GetCurrentWaypoint) -1.0 true true true 0)
        (elif (== (Variables|Default|GetState) 1)
          (bind _returnvalue (Utilities|GetAIController)
            (:Is%20Valid
              (bind _array_element (Utilities|Array|ForEachLoopwithBreak (stale OnPerceptionUpdated(AIPerception) UpdatedActors) :!label _label)
                (:LoopBody
                  (if (<= (Math|Vector|VectorLength (- (Transformation|GetActorLocation (Pawn|GetControlledPawn _returnvalue)) (Transformation|GetActorLocation _array_element))) 1e+02)
                    (goto _label Break)
                    (else
                      (AI|Navigation|MovetoActor _array_element -1.0 true true true 0))))))))))))

(event EventBeginPlay
  (Variables|Default|SetState 0)
  (bind _returnvalue (Utilities|GetAIController)
    (:Is%20Valid
      (bind _outactors (Actor|GetAllActorsOfClass "/Game/Blueprints/BP_Waypoint.BP_Waypoint_C"))
      (Variables|Default|SetCurrentWaypoint (Utilities|Array|Get(acopy) _outactors))
      (Variables|Default|SetCurrentPointID 0)
      (EventDispatchers|BindEventtoReceiveMoveCompleted _returnvalue (delegate Custom|NextRoute))
      ;[0.9949 0.6783 1] Hacer rutas
      (AI|Navigation|MovetoActor (Variables|Default|GetCurrentWaypoint) -1.0 true true true 0))))

(fn ConstructionScript)